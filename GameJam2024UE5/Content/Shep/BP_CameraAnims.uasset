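; BP_CameraAnims is a temporary camera actor that runs a camera animation on the first player controller and takes over the view.
; PlayCameraAnimation starts the animation through the Gameplay Cameras subsystem and blends the view target to this actor.
; EndCameraAnimation stops it non-immediately using the returned handle, blends the view target back to the player controller, then destroys the actor after a delay matching the blend.
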(event `PlayCameraAnimation`
  (bind _returnvalue (`GameplayStatics.GetPlayerController` 0))
  (bind _returnvalue_2 (`GameplayCamerasSubsystem.PlayCameraAnimation` :`self` (subsystem `GameplayCamerasSubsystem`) :`PlayerController` _returnvalue))
  (`PlayerController.SetViewTargetWithBlend` _returnvalue self 1.0 "VTBlend_Linear" 0.0 false))

(event `EndCameraAnimation`
  (`GameplayCamerasSubsystem.StopCameraAnimation` (subsystem `GameplayCamerasSubsystem`) (`GameplayStatics.GetPlayerController` 0) (stale `PlayCameraAnimation` _returnvalue_2) false)
  (`PlayerController.SetViewTargetWithBlend` (`GameplayStatics.GetPlayerController` 0) (`GameplayStatics.GetPlayerController` 0) 1.0 "VTBlend_Linear" 0.0 false)
  (`KismetSystemLibrary.Delay` 1.0)
  (`self.K2_DestroyActor`))

(fn `UserConstructionScript`)